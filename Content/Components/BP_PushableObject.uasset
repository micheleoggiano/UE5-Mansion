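; Pushable block that the player shoves in fixed-distance steps by holding Space and hitting it head-on.
; A valid hit rounds the player's forward vector into a direction, disables movement, attaches the character and plays the push montage.
; A timeline moves the block, repeating while Space stays held, then plays the montage's End section and releases the player.
; CanPush gates steps with aim-input, facing, clearance and floor checks; its falling check sits after the return.
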(event Custom|StopPushing
  (bind _returnvalue (Game|GetPlayerCharacter 0))
  ;[0.15 0.15 0.15 0.5 50] Push Logic
  (Animation|Montage|PlayMontage (Variables|/Script/Engine.Character|GetMesh (Game|GetPlayerCharacter 0)) "/Game/ExportedAnimations/Push/PushMontage.PushMontage" 1.0 0.0 "End"
    (:then
      (Pawn|Components|CharacterMovement|SetMovementMode (Variables|/Script/Engine.Character|GetCharacterMovement _returnvalue) "MOVE_Walking" 0)
      (Transformation|DetachFromActor _returnvalue "KeepWorld" "KeepWorld" "KeepWorld"))))

(event Custom|Push
  ;[0.15 0.15 0.15 0.5 50] Push Logic
  (bind _canpush (CallFunction|CanPush))
  (if _canpush
    (Variables|Default|SetCurrentLocation (Transformation|GetActorLocation))
    (bind _position (Timeline|MoveBlock PlayFromStart)
      (:Update
        (Transformation|SetActorRelativeLocation (+ (* _position (Variables|Default|GetPushableDirection) (Variables|Default|GetTravelDistance)) (Variables|Default|GetCurrentLocation))))
      (:Finished
        (if (Game|Player|IsInputKeyDown (Game|GetPlayerController 0) "SpaceBar")
          (CallFunction|Push)
          (else
            (CallFunction|StopPushing)))))))

(event Collision|EventHit
  (params (MyComp :type Primitive%20Component%20Object%20Reference) (Other :type Actor%20Object%20Reference) (OtherComp :type Primitive%20Component%20Object%20Reference) (bSelfMoved :type Boolean) (HitLocation :type Vector :default "0, 0, 0") (HitNormal :type Vector :default "0, 0, 0") (NormalImpulse :type Vector :default "0, 0, 0") (Hit :type Hit%20Result%20Structure%20%28by%20ref%29))
  (bind _returnvalue (Transformation|GetActorForwardVector Other))
  (bind _returnvalue_2 (Game|GetPlayerCharacter 0))
  (bind _returnvalue_3 (Game|GetPlayerCharacter 0))
  (bind (_x _y _z) (Math|Vector|BreakVector _returnvalue))
  (bind _mesh (Variables|/Script/Engine.Character|GetMesh _returnvalue_3))
  ;[0.15 0.15 0.15 0.5 50] On Hit: Pushable Object
  (if (Game|Player|IsInputKeyDown (Game|GetPlayerController 0) "SpaceBar")
    (if (== (Game|GetPlayerCharacter 0) Other)
      (if (> (Math|Vector|DotProduct HitNormal _returnvalue) 0.93)
        (Variables|Default|SetPushableDirection (Math|Vector|MakeVector (Math|Conversions|ToFloat(Integer) (Math|Float|Round _x)) (Math|Conversions|ToFloat(Integer) (Math|Float|Round _y)) (Math|Conversions|ToFloat(Integer) (Math|Float|Round _z))))
        (bind _canpush (CallFunction|CanPush))
        (if _canpush
          (Pawn|Components|CharacterMovement|DisableMovement (Variables|/Script/Engine.Character|GetCharacterMovement _returnvalue_2))
          (Transformation|AttachActorToActor _returnvalue_2 self "None" "KeepWorld" "KeepWorld" "KeepWorld" true)
          ;[0.15 0.15 0.15 0.5 50] Play Animation Montage
          (if (Class|AnimInstance|IsAnyMontagePlaying (Components|SkeletalMesh|GetAnimInstance _mesh))
            (Utilities|FlowControl|Gate true :!label _label
              (:Exit
                (CallFunction|Push)))
            (else
              (Animation|Montage|PlayMontage _mesh "/Game/ExportedAnimations/Push/PushMontage.PushMontage"
                (:OnNotifyBegin
                  (CallFunction|Push)
                  (goto _label Open))))))))))

(fn ConstructionScript)

(fn CanPush
  (bind _returnvalue (Game|GetPlayerCharacter 0))
  (bind _returnvalue_2 (Transformation|GetActorLocation))
  (bind _returnvalue_3 (Transformation|GetActorLocation))
  (bind _returnvalue_4 (Transformation|GetActorLocation))
  (bind _pushabledirection (Variables|Default|GetPushableDirection))
  (bind _traveldistance (Variables|Default|GetTravelDistance))
  (bind _returnvalue_5 (Transformation|GetActorLocation _returnvalue))
  (bind _returnvalue_6 (* _pushabledirection _traveldistance 1.5))
  (bind _returnvalue_7 (+ _returnvalue_2 "0.000000,0.000000,200.000000"))
  (bind _returnvalue_8 (+ _returnvalue_4 _returnvalue_6 (Math|Vector|MakeVector 0.0 0.0 1e+02)))
  ;[0.15 0.15 0.15 0.5 50] Push Conditions + Resolving Floor Compenetration
  (Utilities|FlowControl|Sequence
    (:then_0
      ;;[0.15 0.15 0.15 0.5 50] 1st Check: Player is not into Aim Mode
      (if (Game|Player|IsInputKeyDown (Game|GetPlayerController 0) "RightMouseButton")
        (LocalVariables|SetLocalCanPush false)))
    (:then_1
      ;;[0.15 0.15 0.15 0.5 50] 2nd Check: Player is Facing the Object
      (bind (_outhit _returnvalue_9) (Collision|LineTraceByChannel _returnvalue_5 (+ _returnvalue_5 (* (Transformation|GetActorForwardVector _returnvalue) 1e+02)) "TraceTypeQuery1" false (Utilities|Array|MakeArray _returnvalue) "None" false))
      (if _returnvalue_9
        (if (not (== (.HitActor (Collision|BreakHitResult _outhit)) self))
          (LocalVariables|SetLocalCanPush false))
        (else
          (LocalVariables|SetLocalCanPush false))))
    (:then_2
      ;;[0.15 0.15 0.15 0.5 50] 3rd Check: The Object Has Room to Move
      (bind _returnvalue_10 (Collision|BoxTraceByChannel (+ _returnvalue_3 (Math|Vector|MakeVector 1e+02 1e+02 1e+02)) (+ _returnvalue_3 (* (Variables|Default|GetPushableDirection) (Variables|Default|GetTravelDistance)) (Math|Vector|MakeVector 1e+02 1e+02 1e+02)) (* (.boxextent (StaticMesh|GetBounds (Variables|/Script/Engine.StaticMeshComponent|GetStaticMesh (Variables|Default|GetCube)))) (Variables|/Script/Engine.SceneComponent|GetRelativeScale3D (Variables|Default|GetCube)) "0.900000,0.900000,0.900000") "0, 0, 0" "TraceTypeQuery1" false 0 "None"))
      (if (not (not _returnvalue_10))
        (LocalVariables|SetLocalCanPush false)))
    (:then_3
      ;;[0.15 0.15 0.15 0.5 50] 4th Check: Floor Under the Object
      (bind _returnvalue_11 (Collision|LineTraceByChannel _returnvalue_8 (+ _returnvalue_8 "0.000000,0.000000,-200.000000") "TraceTypeQuery1" false 0 "None"))
      (if (not _returnvalue_11)
        (LocalVariables|SetLocalCanPush false)))
    (:then_4
      ;;[0.15 0.15 0.15 0.5 50] 5th Check: Anything on Top of the Object
      (bind _returnvalue_12 (Collision|MultiLineTraceByChannel _returnvalue_7 (+ _returnvalue_7 "0.000000,0.000000,200.000000") "TraceTypeQuery1" false 0 "None"))
      (if _returnvalue_12
        (LocalVariables|SetLocalCanPush true)))
    (:then_5
      (return (LocalVariables|GetLocalCanPush)))
    (:then_6
      ;;[0.15 0.15 0.15 0.5 50] 6th Check: Character in "Is Falling" Condition
      (if (AI|Components|NavMovement|IsFalling (Variables|/Script/Engine.Character|GetCharacterMovement (Game|GetPlayerCharacter 0)))
        (LocalVariables|SetLocalCanPush false)))))