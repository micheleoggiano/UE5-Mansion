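; BP_ColorDoor is a double sliding door that opens when used by a BP_PuzzleChecker.
; OnUse plays the ColorDoorOpen timeline, whose alpha slides RDoor and Ldoor apart along relative Y in mirrored motion.
; An alternative Tick-based opening interpolates toward OpenLDoor with VInterpToConstant, negating the left result for RDoor, but sits behind a Gate that nothing opens.
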(event EventOnUse
  (params (Actor :type Actor%20Object%20Reference))
  (Utilities|Casting|CastToBP_PuzzleChecker Actor)
  (bind _alpha (Timeline|ColorDoorOpen Play)
    (:Update
      (Transformation|SetRelativeLocation (Variables|Default|GetRDoor) (Math|Vector|MakeVector 0.0 (Math|Float|Lerp 0.0 1.5e+02 _alpha) 0.0) false false)
      (Transformation|SetRelativeLocation (Variables|Default|GetLdoor) (Math|Vector|MakeVector 0.0 (* (Math|Float|Lerp 0.0 1.5e+02 _alpha) -1.0) 0.0) false false))))

(event EventTick
  (params (DeltaSeconds :type Float%20%28single-precision%29))
  (bind _ldoor (Variables|Default|GetLdoor))
  (bind _openldoor (Variables|Default|GetOpenLDoor))
  (bind _returnvalue (Transformation|GetWorldLocation _ldoor))
  (bind _returnvalue_2 (Transformation|GetWorldLocation _openldoor))
  (bind _returnvalue_3 (Math|Interpolation|VInterptoConstant _returnvalue _returnvalue_2 DeltaSeconds 0.3))
  ;[0.15 0.15 0.15 0.5] Opening with Event Tick, Gate and Vinterp
  (Utilities|FlowControl|Gate true
    (:Exit
      (Transformation|SetWorldLocation (Variables|Default|GetLdoor) _returnvalue_3 false false)
      (Transformation|SetWorldLocation (Variables|Default|GetRDoor) (* _returnvalue_3 -1.0) false false))))

(fn ConstructionScript)